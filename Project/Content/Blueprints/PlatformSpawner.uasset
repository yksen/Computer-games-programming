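; Spawner that places a Platform actor near the player on BeginPlay, through a SpawnPlatform event that can be called again.
; Each platform lands at a random horizontal offset within a distance band around the player's mesh, at a height scaled by Level.
; The new platform receives a reference back to the spawner.
; About half the time a Bullet actor also spawns just above it.
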(event `self.ReceiveBeginPlay`
  (`self.SpawnPlatform`))

(event `SpawnPlatform`
  (bind (_returnvalue_x _returnvalue_y) (`KismetMathLibrary.BreakVector` (`KismetMathLibrary.RandomUnitVector`)))
  (bind _output_get (set `self.Position` (`KismetMathLibrary.MakeVector` (.x (+ (`SceneComponent.K2_GetComponentLocation` (`Character.Mesh` (`GameplayStatics.GetPlayerCharacter` 0))) (* (`KismetMathLibrary.Vector_Normal2D` (`KismetMathLibrary.MakeVector` _returnvalue_x _returnvalue_y)) (`KismetMathLibrary.RandomFloatInRange` 1500.0 1900.0)))) (.y (+ (`SceneComponent.K2_GetComponentLocation` (`Character.Mesh` (`GameplayStatics.GetPlayerCharacter` 0))) (* (`KismetMathLibrary.Vector_Normal2D` (`KismetMathLibrary.MakeVector` _returnvalue_x _returnvalue_y)) (`KismetMathLibrary.RandomFloatInRange` 1500.0 1900.0)))) (`KismetMathLibrary.Conv_IntToDouble` (* (`self.Level`) 500)))))
  (bind _returnvalue (`|SpawnActorFromClass` "/Game/Blueprints/Platform.Platform_C" (`KismetMathLibrary.Conv_VectorToTransform` _output_get) "Undefined" "OverrideRootScale" null null))
  (set `/Game/Blueprints/Platform.Spawner` self _returnvalue)
  (if (> (`KismetMathLibrary.RandomFloat`) 0.5)
    (`|SpawnActorFromClass` "/Game/Blueprints/Bullet.Bullet_C" (`KismetMathLibrary.Conv_VectorToTransform` (+ _output_get (0.0 0.0 200.0))) "Undefined" "OverrideRootScale" null null)))

(fn `UserConstructionScript`)