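; Interactable door Blueprint that swings open and closed around its yaw axis.
; Interact calls Open or Close based on IsOpen and always returns true.
; Open plays and Close reverses one timeline, whose track lerps the Door's relative yaw between CloseRotation and OpenRotation.
; IsOpen flips only when the timeline finishes, so interacting mid-swing repeats the current direction instead of turning the door back.
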(event `Open`
  (bind (_direction _doortrack) (`Timeline|Door Timeline` :!label _label)
    (:`Update`
      (`SceneComponent.K2_SetRelativeRotation` (`self.Door`) (`KismetMathLibrary.MakeRotator` 0.0 0.0 (`KismetMathLibrary.Lerp` (`self.CloseRotation`) (`self.OpenRotation`) _doortrack)) false false))
    (:`Finished`
      (set `self.isOpen` (not (`self.isOpen`))))))

(event `Close`
  (goto _label :!via `Reverse`))

(fn `Interact`
  (params (Interactor :type "Actor Object Reference"))
  (returns (Interacted :type Boolean))
  (if (`self.isOpen`)
    (`self.Close`)
    (else
      (`self.Open`)))
  (return true))

(fn `UserConstructionScript`)